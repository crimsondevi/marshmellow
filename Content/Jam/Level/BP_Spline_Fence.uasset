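; BP_Spline_Fence is a level actor meant to build a fence from spline mesh segments in its construction script.
; With FullLengthMesh on, it adds Y-forward mesh components by spline length over SectionLength, which AllowScale derives from actor Y scale.
; Helper functions compute each segment's local endpoints and length-clamped tangents.
; The calls applying those endpoints and enabling collision are disconnected, so segments never follow the spline.
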(fn `Get End Pos Tangent`
  (params (Index :type Integer))
  (returns (Pos :type "Vector Structure") (Tangent :type "Vector Structure"))
  (bind _spline (`self.Spline`))
  (bind _returnvalue (* (+ Index 1) (`self.SectionLength`)))
  (return (`SplineComponent.GetLocationAtDistanceAlongSpline` _spline _returnvalue "Local") (`KismetMathLibrary.ClampVectorSize` (`SplineComponent.GetTangentAtDistanceAlongSpline` _spline _returnvalue "Local") 0.0 (`self.SectionLength`))))

(fn `Get Start Pos Tangent`
  (params (Index :type Integer))
  (returns (Pos :type "Vector Structure") (Tangent :type "Vector Structure"))
  (bind _sectionlength (`self.SectionLength`))
  (bind _spline (`self.Spline`))
  (bind _returnvalue (* Index _sectionlength))
  (return (`SplineComponent.GetLocationAtDistanceAlongSpline` _spline _returnvalue "Local") (`KismetMathLibrary.ClampVectorSize` (`SplineComponent.GetTangentAtDistanceAlongSpline` _spline _returnvalue "Local") 0.0 _sectionlength)))

(fn `UserConstructionScript`
  (bind (_returnvalue_x _returnvalue_y) (`KismetMathLibrary.BreakVector` (`self.GetActorScale3D`)))
  (if (`self.AllowScale?`)
    (set `self.SectionLength` (* _returnvalue_y 100.0)))
  (if (`self.FullLengthMesh?`)
    (for _index (range (+ (`KismetMathLibrary.FTrunc` (/ (`SplineComponent.GetSplineLength` (`self.Spline`)) (`self.SectionLength`))) 1))
      (set `self.LoopIndex` _index)
      (bind _returnvalue (`AddComponent|NODE_AddSplineMeshComponent-0`))
      (`StaticMeshComponent.SetStaticMesh` _returnvalue (`self.SplineMesh`))
      (`SplineMeshComponent.SetForwardAxis` _returnvalue "Y" true)
      (bind (_pos _tangent) (`self.Get Start Pos Tangent` (`self.LoopIndex`)))
      (bind (_pos_2 _tangent_2) (`self.Get End Pos Tangent` (`self.LoopIndex`))))))